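; GA_EnemyPistolAbility is a gameplay ability for the pistol enemy, providing helper functions with no active activation logic in the event graph.
; GetEnemy casts the owning actor to BP_PistolEnemy and caches it.
; GetLineTrace, copied from the player pistol ability, still traces from the player's camera along its forward vector out to weapon range on Visibility, returning the hit actor or cancelling the ability.
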(fn `GetEnemy`
  (bind _returnvalue_owneractor (break `GameplayAbilityActorInfo` (`self.GetActorInfo`)))
  (`/Engine/EditorBlueprintResources/StandardMacros.IsValid` (`self.PistolEnemy`)
    (:`Is Valid`
      _)
    (:`Is Not Valid`
      (bind _asbp_pistol_enemy (cast `/Game/RetroFPS/Blueprints/Enemies/BP_PistolEnemy` _returnvalue_owneractor))
      (set `self.PistolEnemy` _asbp_pistol_enemy)))
  (return))

(fn `GetLineTrace`
  (returns (Actor :type "Actor Object Reference"))
  (bind _camera (`/Game/RetroFPS/Blueprints/Player/BP_FPSPlayer.Camera` (`self.Player`)))
  (bind _returnvalue (`SceneComponent.K2_GetComponentLocation` _camera))
  (bind _outhit (`KismetSystemLibrary.LineTraceSingle` _returnvalue (+ _returnvalue (* (`KismetMathLibrary.GetForwardVector` (`SceneComponent.K2_GetComponentRotation` _camera)) (`self.Weapon Range`))) "TraceTypeQuery1")) ; (Copied from GA_PlayerPistolAbility)
  (bind (_bblockinghit _binitialoverlap _time _distance _location _impactpoint _normal _impactnormal _physmat _hitactor) (`GameplayStatics.BreakHitResult` _outhit))
  (`/Engine/EditorBlueprintResources/StandardMacros.IsValid` _hitactor
    (:`Is Valid`
      (return _hitactor))
    (:`Is Not Valid`
      (`self.K2_CancelAbility`))))