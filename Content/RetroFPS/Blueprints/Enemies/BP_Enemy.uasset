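; Retro FPS enemy character drawn as a billboard flipbook sprite with eight-directional facing, driven by an AI behavior tree.
; Each tick it yaws the sprite toward the camera, then picks a walk or idle flipbook from velocity and the player's angle relative to its facing.
; Damage and death override the directional flipbooks; death also stops AI logic and capsule collision.
; Melee and ranged attacks only print debug text.
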(event `self.ReceiveBeginPlay`
  (bind _asbp_retro_fpsenemy_ai (cast `/Game/RetroFPS/Blueprints/Enemies/AI/BP_RetroFPSEnemyAI` (`self.GetController`)))
  (`AIController.RunBehaviorTree` _asbp_retro_fpsenemy_ai (`self.BehaviourTree`)))

(event `self.ReceiveTick`
  (params (DeltaSeconds :type "Float (single-precision)"))
  (`self.SpriteFacePlayer`
    (:`Out`
      (if (not (or (`self.IsDead`) (`self.PauseAngleCalculations`)))
        (`self.GetEnemyAngle`
          (:`Out`
            (`self.CheckIfWalking`
              (:`Out`
                (`self.CalculateFlipbook`)))))))))

(event `self.TakeDamage`
  (params (CueData :type "GameplayCueParameters Structure"))
  (bind _enemy (`self.Enemy`))
  (`parent.TakeDamage` CueData)
  (if (not (`self.IsDead`))
    (set `self.PauseAngleCalculations` true)
    (`PaperFlipbookComponent.SetFlipbook` _enemy (`self.Damaged`))
    (`KismetSystemLibrary.Delay` (`PaperFlipbookComponent.GetFlipbookLength` _enemy))
    (set `self.PauseAngleCalculations` false) ; (resume sprite facing player)
  ))

(event `self.KillCharacter`
  (bind _enemy (`self.Enemy`))
  (`parent.KillCharacter`)
  (bind _asbp_retro_fpsenemy_ai (cast `/Game/RetroFPS/Blueprints/Enemies/AI/BP_RetroFPSEnemyAI` (`self.GetController`)))
  (`BrainComponent.StopLogic` (`AIController.BrainComponent` _asbp_retro_fpsenemy_ai) "")
  (set `self.IsDead` true)
  (`PrimitiveComponent.SetCollisionEnabled` (`self.CapsuleComponent`) "NoCollision")
  (`PaperFlipbookComponent.SetFlipbook` _enemy (`self.Dying`))
  (`KismetSystemLibrary.Delay` (`PaperFlipbookComponent.GetFlipbookLength` _enemy))
  (`PaperFlipbookComponent.SetFlipbook` (`self.Enemy`) (`self.Dead`)))

(event `MeleeAttack`
  (`KismetSystemLibrary.PrintString` "melee attack!"))

(event `RangedAttack`
  (`KismetSystemLibrary.PrintString` "Ranged Attack!"))

(fn `SetFlipbook`
  (params (Walking :type "PaperFlipbook Object Reference") (Idle :type "PaperFlipbook Object Reference"))
  (bind _enemy (`self.Enemy`))
  (if (`self.IsWalking`)
    (`PaperFlipbookComponent.SetFlipbook` _enemy Walking)
    (else
      (`PaperFlipbookComponent.SetFlipbook` _enemy Idle)))
  (return))

(fn `UserConstructionScript`)