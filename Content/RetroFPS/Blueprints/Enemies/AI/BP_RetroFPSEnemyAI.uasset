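; Enemy AI for RetroFPS that turns perception updates on Player-tagged actors into Blackboard state.
; Sensing the player sets CanSeeTarget and TargetActor and cancels any pending lost-sight timer.
; Losing the player clears CanSeeTarget at once but keeps TargetActor until a delayed LostSight timer empties it, giving the enemy a short memory of its target.
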(event `self.AIPerception.OnTargetPerceptionUpdated`
  (params (Actor :type "Actor Object Reference") (Stimulus :type "AIStimulus Structure"))
  (bind _output_get (set `self.PerceivedActor` Actor))
  (if (`self.ActorHasTag` _output_get "Player")
    (if Stimulus_bSuccessfullySensed
      (`KismetSystemLibrary.K2_ClearAndInvalidateTimerHandle` (`self.LostSightTimer`))
      (`self.UpdateSightKey` true)
      (`self.UpdateTargetKey` (`self.PerceivedActor`))
      (else
        (bind _returnvalue (`KismetSystemLibrary.K2_SetTimerDelegate` (delegate `Lost Sight`) 8.0))
        (set `self.LostSightTimer` _returnvalue)
        (`self.UpdateSightKey` false)))))

(event `Lost Sight`
  (`self.UpdateTargetKey` null) ; Lose the target actor
)

(fn `UpdateSightKey`
  (params (HasLineOfSight :type Boolean))
  (`BlackboardComponent.SetValueAsBool` (`AIBlueprintHelperLibrary.GetBlackboard` null) "CanSeeTarget" HasLineOfSight))

(fn `UpdateTargetKey`
  (params (TargetActor :type "Actor Object Reference"))
  (`BlackboardComponent.SetValueAsObject` (`AIBlueprintHelperLibrary.GetBlackboard` null) "TargetActor" TargetActor))

(fn `UserConstructionScript`)